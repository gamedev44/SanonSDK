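; Tank shell projectile that damages and explodes on hit, then destroys itself after a short delay, or expires with its lifespan.
; ApplyDamage tries full radial damage, falling back to point damage on the hit actor, except MANPADS-type hits on landscape.
; Explosion Niagara effect and sound route through Server and All events for replication.
; A large shared vehicle interface is mostly stubbed, identifying it as a shell and supplying its damage.
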(event Custom|SpawnNS_Explosion
  (params (SystemTemplate :type Niagara%20System%20Object%20Reference) (Location :type Vector) (Sound :type Sound%20Base%20Object%20Reference))
  (CallFunction|SpawnNSExplosion-Server SystemTemplate Location Sound))

(event Custom|SpawnNS_Explosion%20-%20Server
  (params (SystemTemplate :type Niagara%20System%20Object%20Reference) (Location :type Vector) (Sound :type Sound%20Base%20Object%20Reference))
  (CallFunction|SpawnNSExplosion-All SystemTemplate Location Sound))

(event Custom|SpawnNS_Explosion%20-%20All
  (params (SystemTemplate :type Niagara%20System%20Object%20Reference) (Location :type Vector) (Sound :type Sound%20Base%20Object%20Reference))
  (Niagara|SpawnSystematLocation SystemTemplate Location)
  (Audio|PlaySoundatLocation Sound Location "0, 0, 0" 1.0 1.0 0.0 0 0 0 0))

(event EventBeginPlay
  (Actor|SetLifeSpan (Variables|Settings|GetLifespan)))

(event Collision|EventHit
  (params (MyComp :type Primitive%20Component%20Object%20Reference) (Other :type Actor%20Object%20Reference) (OtherComp :type Primitive%20Component%20Object%20Reference) (bSelfMoved :type Boolean) (HitLocation :type Vector :default "0, 0, 0") (HitNormal :type Vector :default "0, 0, 0") (NormalImpulse :type Vector :default "0, 0, 0") (Hit :type Hit%20Result%20Structure%20%28by%20ref%29))
  (CallFunction|ApplyDamage HitLocation Other HitNormal Hit)
  (Utilities|FlowControl|Delay 0.2)
  (Actor|DestroyActor))

(fn ConstructionScript)

(fn TypeOfShell
  (return "NewEnumerator2"))

(fn GetBlackboardRef
  (return 0))

(fn GetPointtoShot
  (return 0))

(fn IsTankActive
  (return false))

(fn GetDriverInside
  (return 0))

(fn GetLastActiveWeapon
  (return "NewEnumerator0"))

(fn GetCountOfSmokes
  (return 0))

(fn GetCountOfMachineGun
  (return 0))

(fn GetActiveCamera
  (return "NewEnumerator0"))

(fn GetAllWeapons
  (return "NewEnumerator0"))

(fn GetCountofShells
  (return 0))

(fn GetHealth
  (return 0.0 0.0))

(fn IsHeatTrap
  (return false))

(fn GetDetectionDistance[Fighter]
  (return 0.0))

(fn GetBody
  (return 0 0))

(fn GetSpeed
  (return 0.0))

(fn GetTarget
  (return 0))

(fn Sensible
  (return false))

(fn GetTeam
  (return "NewEnumerator2"))

(fn GetTurret
  (return 0))

(fn GetLeftWheels
  (return 0))

(fn GetRightWheels
  (return 0))

(fn GetSplineL
  (return 0))

(fn GetSplineR
  (return 0))

(fn GetTrackL
  (return 0))

(fn GetTrackR
  (return 0))

(fn GetSuspensions
  (return 0))

(fn GetBarrel
  (return 0))

(fn IsTank
  (return false))

(fn GetArrowMinigun
  (return 0))

(fn GetTankSettings
  (return ""))

(fn IsAiming1)

(fn GetMiniGunTurret
  (return 0))

(fn GetArrowBarrel
  (return 0))

(fn PlaceforShotSound
  (return 0))

(fn IsDestroyed
  (return false))

(fn GetMainShotParticle
  (return 0))

(fn GetSecondShotParticle
  (return 0))

(fn GetArrowSmoke
  (return 0))

(fn GetBodyCamera
  (return 0))

(fn GetCameraTurret
  (return 0))

(fn GetCameraAimInside
  (return 0))

(fn GetCameraMinigun
  (return 0))

(fn GetMainSpringArm
  (return 0))

(fn GetDefaultAim
  (return 0))

(fn GetPredictAim
  (return 0))

(fn GetMinigunAim
  (return 0))

(fn GetPlaceforAmmunitionExplosionParticle
  (return 0))

(fn GetAudioAmmunitionExplosion
  (return 0))

(fn GetDestroyedTankParticle
  (return 0))

(fn GetDestroyedTankSmokeParticle
  (return 0))

(fn GetHitWidget
  (return 0))

(fn GetRicochetSound
  (return 0))

(fn TankStarted
  (return false))

(fn IamParent
  (return false))

(fn BulletDamage
  (return 0.0))

(fn GetSusp
  (return 0))

(fn GetLastWheels
  (return 0))

(fn GetMinigunShellPlace
  (return 0))

(fn GetBreakThroughSound
  (return 0))

(fn GetShotAudio
  (return 0))

(fn GetMainCamera
  (return 0))

(fn IsVehicleTarget
  (return false))

(fn GetPawnType
  (return "NewEnumerator1"))

(fn GetShellDamage
  (return 1e+03))

(fn GetVehicleHealthInfo
  (return ""))

(fn GetPlaneSettings
  (return ""))

(fn GetParentOwner
  (bind _driver (Class|BPIVehicles|GetDriver(Message) (Components|GetOwner)))
  (return _driver))

(fn IsItTrack
  (return false))

(fn IsComponentAllright
  (return false))

(fn GetCountOfCannonShells
  (return 0))

(fn GetSmokeSettings
  (return ""))

(fn GetMinigunSettings
  (return ""))

(fn IsAiming
  (return false))

(fn GetCannonSound
  (return 0))

(fn GetCannonSettings
  (return ""))

(fn CanShot?
  (return false))

(fn IsTankValid
  (return false))

(fn GetReloadTime
  (return 0.0))

(fn ApplyDamage
  (params (HitLocation :type Vector%20%28by%20ref%29) (Other :type Actor%20Object%20Reference) (HitNormal :type Vector) (Hit :type Hit%20Result%20Structure%20%28by%20ref%29))
  (LocalVariables|SetHL HitLocation)
  (LocalVariables|SetHN HitNormal)
  (bind _damage (CallFunction|GetShellDamage))
  (LocalVariables|SetDamageL _damage)
  (bind _returnvalue (Game|Damage|ApplyRadialDamage (LocalVariables|GetDamageL) (LocalVariables|GetHL) 5e+02 (Variables|Settings|GetDamageTypeClass) (Utilities|Array|MakeArray (Components|GetOwner)) self (Pawn|GetController (.AsPawn (Utilities|Casting|CastToPawn (Components|GetOwner)))) true "ECC_GameTraceChannel4"))
  (if _returnvalue
    (CallFunction|SpawnNSExplosion (Variables|Settings|GetNS_Hit) (Transformation|GetActorLocation) "/Game/ModernRPG/Tanks/Sounds/Noise/Effects/SC_ShellHit.SC_ShellHit")
    (else
      (Utilities|Casting|CastToBPDT_MANPADSClass (Variables|Settings|GetDamageTypeClass)
        (:then
          (Utilities|Casting|CastToLandscape Other
            (:then
              (CallFunction|SpawnNSExplosion (Variables|Settings|GetNS_Hit) (Transformation|GetActorLocation) "/Game/ModernRPG/Tanks/Sounds/Noise/Effects/SC_ShellHit.SC_ShellHit"))
            (:CastFailed
              (Game|Damage|ApplyPointDamage Other (LocalVariables|GetDamageL) (LocalVariables|GetHN) Hit (Pawn|GetController (.AsPawn (Utilities|Casting|CastToPawn (Components|GetOwner)))) (Components|GetOwner) (Variables|Settings|GetDamageTypeClass) :!label _label)
              (CallFunction|SpawnNSExplosion (Variables|Settings|GetNS_Hit) (Transformation|GetActorLocation) "/Game/ModernRPG/Tanks/Sounds/Noise/Effects/SC_ShellHit.SC_ShellHit"))))
        (:CastFailed
          (goto _label))))))

(fn IsShell
  (return true))

(fn GetName
  (return ""))

(fn IsAlive?
  (return false))

(fn IsUsingAlternativeSkeleton?
  (return "NewEnumerator0"))

(fn Person?
  (return false))