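; Actor component that gives non-AI vehicles rocket launcher target lock-on, destroying itself on AI owners.
; While searching, a looping timer gathers live vehicles overlapping the owner's "Locator" boxes, filters them by line-of-sight trace and picks the nearest.
; The chosen target is passed to the owner and highlighted through indicator widgets in "Mark"-tagged child actors.
; Events also show or hide these widgets and notify the target's widget of rocket launches.
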(event Custom|FindTarget
  ;[1 1 1] Find target
  (CallFunction|FindAllTargets-Server))

(event Custom|HideWidgets%20-%20OC
  ;[1 1 1] Show widgets of each actor
  (for _array_element (CallFunction|FindArray)
    (bind _outactors (Actor|GetAllActorsOfClass _array_element))
    (if (Utilities|Array|IsValidIndex _outactors)
      (for _array_element_2 _outactors
        (for _array_element_3 (Actor|GetComponentsbyTag _array_element_2 "/Script/Engine.ChildActorComponent" "Mark")
          (Utilities|IsValid (Variables|/Script/Engine.ChildActorComponent|GetChildActor _array_element_3)
            (:Is%20Valid
              (Utilities|IsValid (.AsBP%20Target%20Indicator (Utilities|Casting|CastToBP_TargetIndicator (Variables|/Script/Engine.ChildActorComponent|GetChildActor _array_element_3)))
                (:Is%20Valid
                  (Utilities|IsValid (UserInterface|GetUserWidgetObject (Variables|/Game/ModernRPG/General/Blueprints/Weapon/RL/BP_TargetIndicator.BP_TargetIndicator_C|GetWB (.AsBP%20Target%20Indicator (Utilities|Casting|CastToBP_TargetIndicator (Variables|/Script/Engine.ChildActorComponent|GetChildActor _array_element_3)))))
                    (:Is%20Valid
                      (Class|BPIWidgets|ControlRL(Message) (UserInterface|GetUserWidgetObject (Variables|/Game/ModernRPG/General/Blueprints/Weapon/RL/BP_TargetIndicator.BP_TargetIndicator_C|GetWB (.AsBP%20Target%20Indicator (Utilities|Casting|CastToBP_TargetIndicator (Variables|/Script/Engine.ChildActorComponent|GetChildActor _array_element_3))))) "Hidden")
                      (Class|BPIWidgets|ControlMarked(Message) (UserInterface|GetUserWidgetObject (Variables|/Game/ModernRPG/General/Blueprints/Weapon/RL/BP_TargetIndicator.BP_TargetIndicator_C|GetWB (.AsBP%20Target%20Indicator (Utilities|Casting|CastToBP_TargetIndicator (Variables|/Script/Engine.ChildActorComponent|GetChildActor _array_element_3))))) false))))))))))))

(event Custom|ShowWidgets%20-%20OC
  ;[1 1 1] Show widgets of each actor
  (for _array_element (CallFunction|FindArray)
    (bind _outactors (Actor|GetAllActorsOfClass _array_element))
    (if (Utilities|Array|IsValidIndex _outactors)
      (for _array_element_2 _outactors
        (if (!= _array_element_2 (Components|GetOwner))
          (bind _result (Class|BPICharacter|IsAlive?(Message) _array_element_2))
          (if _result
            (for _array_element_3 (Actor|GetComponentsbyTag _array_element_2 "/Script/Engine.ChildActorComponent" "Mark")
              (Utilities|IsValid (Variables|/Script/Engine.ChildActorComponent|GetChildActor _array_element_3)
                (:Is%20Valid
                  (Utilities|IsValid (.AsBP%20Target%20Indicator (Utilities|Casting|CastToBP_TargetIndicator (Variables|/Script/Engine.ChildActorComponent|GetChildActor _array_element_3)))
                    (:Is%20Valid
                      (Utilities|IsValid (UserInterface|GetUserWidgetObject (Variables|/Game/ModernRPG/General/Blueprints/Weapon/RL/BP_TargetIndicator.BP_TargetIndicator_C|GetWB (.AsBP%20Target%20Indicator (Utilities|Casting|CastToBP_TargetIndicator (Variables|/Script/Engine.ChildActorComponent|GetChildActor _array_element_3)))))
                        (:Is%20Valid
                          (Class|BPIWidgets|ControlRL(Message) (UserInterface|GetUserWidgetObject (Variables|/Game/ModernRPG/General/Blueprints/Weapon/RL/BP_TargetIndicator.BP_TargetIndicator_C|GetWB (.AsBP%20Target%20Indicator (Utilities|Casting|CastToBP_TargetIndicator (Variables|/Script/Engine.ChildActorComponent|GetChildActor _array_element_3))))) "Visible")
                          (Default|EventSetupRef (.AsWB%20RLIndicator (Utilities|Casting|CastToWB_RLIndicator (UserInterface|GetUserWidgetObject (Variables|/Game/ModernRPG/General/Blueprints/Weapon/RL/BP_TargetIndicator.BP_TargetIndicator_C|GetWB (.AsBP%20Target%20Indicator (Utilities|Casting|CastToBP_TargetIndicator (Variables|/Script/Engine.ChildActorComponent|GetChildActor _array_element_3))))))) _array_element_2))))))))))))))

(event Custom|FindTarget%20-%20Server
  (params (TargetRocketLauncher :type Actor%20Object%20Reference))
  ;[1 1 1] Find target
  (Utilities|IsValid (Variables|Default|GetTargetRocketLauncher)
    (:Is%20Valid
      (Utilities|IsValid TargetRocketLauncher
        (:Is%20Valid
          (if (== (Variables|Default|GetTargetRocketLauncher) TargetRocketLauncher)
            _
            (else
              (CallFunction|Unmark-OC (Variables|Default|GetTargetRocketLauncher))))
          (bind _output_get (Variables|Default|SetTargetRocketLauncher TargetRocketLauncher :!label _label))
          (CallFunction|Mark-OC _output_get)
          (Class|BPIPlayerInfo|SetTarget(Message) (Components|GetOwner) (Variables|Default|GetTargetRocketLauncher)))
        (:Is%20Not%20Valid
          (CallFunction|Unmark-OC (Variables|Default|GetTargetRocketLauncher) :!label _label_2)
          (Variables|Default|SetTargetRocketLauncher 0)
          (Class|BPIPlayerInfo|SetTarget(Message) (Components|GetOwner))
          (for _array_element (CallFunction|FindArray)
            (bind _outactors (Actor|GetAllActorsOfClass _array_element))
            (if (Utilities|Array|IsValidIndex _outactors)
              (for _array_element_2 _outactors
                (CallFunction|Unmark-OC _array_element_2)))))))
    (:Is%20Not%20Valid
      (Utilities|IsValid TargetRocketLauncher
        (:Is%20Valid
          (goto _label))
        (:Is%20Not%20Valid
          (goto _label_2))))))

(event Custom|Unmark%20-%20OC
  (params (Target :type Actor%20Object%20Reference))
  (bind _returnvalue (Actor|GetComponentsbyTag Target "/Script/Engine.ChildActorComponent" "Mark"))
  ;[1 1 1] Mark&Unmark
  (Utilities|IsValid Target
    (:Is%20Valid
      (if (Utilities|Array|IsValidIndex _returnvalue)
        (for _array_element _returnvalue
          (Utilities|IsValid _array_element
            (:Is%20Valid
              (Utilities|IsValid (.AsBP%20Target%20Indicator (Utilities|Casting|CastToBP_TargetIndicator (Variables|/Script/Engine.ChildActorComponent|GetChildActor _array_element)))
                (:Is%20Valid
                  (Utilities|IsValid (UserInterface|GetUserWidgetObject (Variables|/Game/ModernRPG/General/Blueprints/Weapon/RL/BP_TargetIndicator.BP_TargetIndicator_C|GetWB (.AsBP%20Target%20Indicator (Utilities|Casting|CastToBP_TargetIndicator (Variables|/Script/Engine.ChildActorComponent|GetChildActor _array_element)))))
                    (:Is%20Valid
                      (Class|BPIWidgets|ControlMarked(Message) (UserInterface|GetUserWidgetObject (Variables|/Game/ModernRPG/General/Blueprints/Weapon/RL/BP_TargetIndicator.BP_TargetIndicator_C|GetWB (.AsBP%20Target%20Indicator (Utilities|Casting|CastToBP_TargetIndicator (Variables|/Script/Engine.ChildActorComponent|GetChildActor _array_element))))) false))))))))
        (Class|BPIRocketLauncher|TargetLocked(Message) (Components|GetOwner) false)))))

(event Custom|SetupWidgetOwners%20-%20OC
  ;[1 1 1] Setup owners
  (for _array_element (CallFunction|FindArray)
    (bind _outactors (Actor|GetAllActorsOfClass _array_element))
    (if (Utilities|Array|IsValidIndex _outactors)
      (for _array_element_2 _outactors
        (if (!= _array_element_2 (Components|GetOwner))
          (bind _result (Class|BPICharacter|IsAlive?(Message) _array_element_2))
          (if _result
            (for _array_element_3 (Actor|GetComponentsbyTag _array_element_2 "/Script/Engine.ChildActorComponent" "Mark")
              (Utilities|IsValid (Variables|/Script/Engine.ChildActorComponent|GetChildActor _array_element_3)
                (:Is%20Valid
                  (Utilities|IsValid (.AsBP%20Target%20Indicator (Utilities|Casting|CastToBP_TargetIndicator (Variables|/Script/Engine.ChildActorComponent|GetChildActor _array_element_3)))
                    (:Is%20Valid
                      (Utilities|IsValid (UserInterface|GetUserWidgetObject (Variables|/Game/ModernRPG/General/Blueprints/Weapon/RL/BP_TargetIndicator.BP_TargetIndicator_C|GetWB (.AsBP%20Target%20Indicator (Utilities|Casting|CastToBP_TargetIndicator (Variables|/Script/Engine.ChildActorComponent|GetChildActor _array_element_3)))))
                        (:Is%20Valid
                          (Default|EventSetupRef (.AsWB%20RLIndicator (Utilities|Casting|CastToWB_RLIndicator (UserInterface|GetUserWidgetObject (Variables|/Game/ModernRPG/General/Blueprints/Weapon/RL/BP_TargetIndicator.BP_TargetIndicator_C|GetWB (.AsBP%20Target%20Indicator (Utilities|Casting|CastToBP_TargetIndicator (Variables|/Script/Engine.ChildActorComponent|GetChildActor _array_element_3))))))) _array_element_2)
                          (Default|SetWidgetOwner-OC (.AsWB%20RLIndicator (Utilities|Casting|CastToWB_RLIndicator (UserInterface|GetUserWidgetObject (Variables|/Game/ModernRPG/General/Blueprints/Weapon/RL/BP_TargetIndicator.BP_TargetIndicator_C|GetWB (.AsBP%20Target%20Indicator (Utilities|Casting|CastToBP_TargetIndicator (Variables|/Script/Engine.ChildActorComponent|GetChildActor _array_element_3))))))) _array_element_2))))))))))))))

(event Custom|Mark%20-%20OC
  (params (Target :type Actor%20Object%20Reference))
  (bind _returnvalue (Actor|GetComponentsbyTag Target "/Script/Engine.ChildActorComponent" "Mark"))
  ;[1 1 1] Mark&Unmark
  (if (Utilities|Array|IsValidIndex _returnvalue)
    (for _array_element _returnvalue
      (Utilities|IsValid (Variables|/Script/Engine.ChildActorComponent|GetChildActor _array_element)
        (:Is%20Valid
          (Utilities|IsValid (.AsBP%20Target%20Indicator (Utilities|Casting|CastToBP_TargetIndicator (Variables|/Script/Engine.ChildActorComponent|GetChildActor _array_element)))
            (:Is%20Valid
              (Utilities|IsValid (UserInterface|GetUserWidgetObject (Variables|/Game/ModernRPG/General/Blueprints/Weapon/RL/BP_TargetIndicator.BP_TargetIndicator_C|GetWB (.AsBP%20Target%20Indicator (Utilities|Casting|CastToBP_TargetIndicator (Variables|/Script/Engine.ChildActorComponent|GetChildActor _array_element)))))
                (:Is%20Valid
                  (Class|BPIWidgets|ControlMarked(Message) (UserInterface|GetUserWidgetObject (Variables|/Game/ModernRPG/General/Blueprints/Weapon/RL/BP_TargetIndicator.BP_TargetIndicator_C|GetWB (.AsBP%20Target%20Indicator (Utilities|Casting|CastToBP_TargetIndicator (Variables|/Script/Engine.ChildActorComponent|GetChildActor _array_element))))) true))))))))
    (Class|BPIRocketLauncher|TargetLocked(Message) (Components|GetOwner) true)))

(event Custom|Shot%20-%20OC
  (params (Rocket :type Actor%20Object%20Reference))
  ;[1 1 1] Shot a rocket
  (Utilities|IsValid (Variables|Default|GetTargetRocketLauncher)
    (:Is%20Valid
      (bind _mark (Class|BPIInteract|GetMarkUI(Message) (Variables|Default|GetTargetRocketLauncher)))
      (Utilities|IsValid _mark
        (:Is%20Valid
          (bind _asbp_target_indicator (Utilities|Casting|CastToBP_TargetIndicator (Variables|/Script/Engine.ChildActorComponent|GetChildActor _mark)))
          (bind _aswb_rlindicator (Utilities|Casting|CastToWB_RLIndicator (UserInterface|GetUserWidgetObject (Variables|/Game/ModernRPG/General/Blueprints/Weapon/RL/BP_TargetIndicator.BP_TargetIndicator_C|GetWB _asbp_target_indicator))))
          (Default|RocketLaunchedOC _aswb_rlindicator Rocket (Variables|Default|GetTargetRocketLauncher)))))))

(event Custom|ShowHealthWidget%20-%20OC
  ;[1 1 1] Setup owners
  (for _array_element (Actor|GetComponentsbyTag (Components|GetOwner) "/Script/Engine.ChildActorComponent" "Mark")
    (Utilities|IsValid (Variables|/Script/Engine.ChildActorComponent|GetChildActor _array_element)
      (:Is%20Valid
        (Utilities|IsValid (.AsBP%20Target%20Indicator (Utilities|Casting|CastToBP_TargetIndicator (Variables|/Script/Engine.ChildActorComponent|GetChildActor _array_element)))
          (:Is%20Valid
            (Utilities|IsValid (UserInterface|GetUserWidgetObject (Variables|/Game/ModernRPG/General/Blueprints/Weapon/RL/BP_TargetIndicator.BP_TargetIndicator_C|GetWB (.AsBP%20Target%20Indicator (Utilities|Casting|CastToBP_TargetIndicator (Variables|/Script/Engine.ChildActorComponent|GetChildActor _array_element)))))
              (:Is%20Valid
                (Default|ShowHealthWidget (.AsWB%20RLIndicator (Utilities|Casting|CastToWB_RLIndicator (UserInterface|GetUserWidgetObject (Variables|/Game/ModernRPG/General/Blueprints/Weapon/RL/BP_TargetIndicator.BP_TargetIndicator_C|GetWB (.AsBP%20Target%20Indicator (Utilities|Casting|CastToBP_TargetIndicator (Variables|/Script/Engine.ChildActorComponent|GetChildActor _array_element))))))))))))))))

(event Custom|FindAllTargets%20-%20Server
  ;[1 1 1] Find target
  (Utilities|Array|Clear (Variables|Default|GetTargets))
  (for _array_element (Variables|Detector|GetLocators)
    (CallFunction|AddVehicle _array_element))
  (Variables|Default|SettargetCaptured true)
  (CallFunction|FindTarget-Server (CallFunction|FindNearest)))

(event EventBeginPlay
  (CallFunction|SetupWidgetOwners-OC)
  (CallFunction|Initializing))

(event EventFindTargetStart
  ;[1 1 1] Find target
  (Utilities|Array|Clear (Variables|Default|GetTargets))
  (Variables|Default|SettargetCaptured false)
  (Variables|Default|SetTimer 0)
  (bind _returnvalue (Utilities|Time|SetTimerbyEvent (delegate Custom|FindTarget) 0.5 true))
  (Variables|Default|SetFindTargetTimer _returnvalue)
  (if (Ability|HasAuthority (Components|GetOwner))
    (CallFunction|ShowWidgets-OC)))

(event EventFindTargetStop
  ;[1 1 1] Stop trying to find actor
  (Utilities|Time|PauseTimerbyHandle (Variables|Default|GetFindTargetTimer))
  (CallFunction|HideWidgets-OC)
  (CallFunction|Unmark-OC (Variables|Default|GetTargetRocketLauncher))
  (Variables|Default|SetTargetRocketLauncher 0)
  (Class|BPIPlayerInfo|SetTarget(Message) (Components|GetOwner) (Variables|Default|GetTargetRocketLauncher)))

(fn Initializing
  (bind _isai_ (Class|BPIPlayerInfo|IsAI?(Message) (Components|GetOwner)))
  (if _isai_
    (Components|DestroyComponent)
    (else
      (if (Variables|/Game/ModernRPG/General/Blueprints/GameInstance/BP_GameInstanceinfo.BP_GameInstanceinfo_C|GetSoloPlay? (.AsBP%20Game%20Instanceinfo (Utilities|Casting|CastToBP_GameInstanceinfo (Game|GetGameInstance))))
        _
        (else
          _))
      (bind _s_fightersettings (Class|BPIPlayerInfo|GetFighterSettings(Message) (Components|GetOwner)))
      (Variables|Default|SetS_Fighter _s_fightersettings)
      (Variables|Detector|SetLocators (Actor|GetComponentsbyTag (Components|GetOwner) "/Script/Engine.BoxComponent" "Locator"))
      (Variables|Default|SetCanTick true))))

(fn AddVehicle
  (params (Target :type Primitive%20Component%20Object%20Reference))
  (for _array_element (CallFunction|FindArray)
    (if (Utilities|Array|IsValidIndex (Collision|GetOverlappingActors Target _array_element :!class /Script/Engine.PrimitiveComponent))
      (for _array_element_2 (Collision|GetOverlappingActors Target _array_element :!class /Script/Engine.PrimitiveComponent)
        (if (!= _array_element_2 (Components|GetOwner))
          (bind _istarget (Class|BPIAI|IsVehicleTarget(Message) _array_element_2))
          (if _istarget
            (bind _result (Class|BPICharacter|IsAlive?(Message) _array_element_2))
            (if _result
              (bind _billboard (Class|BPIAI|GetPointtoShot(Message) _array_element_2))
              (if (Utilities|IsValid _billboard)
                (bind _bodyskeletal (Class|BPIAI|GetBody(Message) (Components|GetOwner)))
                (bind (_outhit _returnvalue) (Collision|LineTraceByChannel (Transformation|GetWorldLocation _bodyskeletal) (Transformation|GetWorldLocation _billboard) "TraceTypeQuery1" false (Utilities|Array|MakeArray (Components|GetOwner (Components|GetOwner)) (Components|GetOwner)) "None"))
                (if _returnvalue
                  (if (== (.HitActor (Collision|BreakHitResult _outhit)) _array_element_2)
                    (bind _aspawn (Utilities|Casting|CastToPawn _array_element_2)
                      (:then
                        (Utilities|Array|AddUnique (Variables|Default|GetTargets) _aspawn))
                      (:CastFailed
                        (bind _owner (Class|BPIVehicles|GetParentOwner(Message) _array_element_2))
                        (bind _aspawn_2 (Utilities|Casting|CastToPawn _owner))
                        (Utilities|Array|AddUnique (Variables|Default|GetTargets) _aspawn_2)))
                    (else
                      (bind _owner_2 (Class|BPIVehicles|GetParentOwner(Message) (.HitActor (Collision|BreakHitResult _outhit))))
                      (if (== _owner_2 _array_element_2)
                        (bind _aspawn_3 (Utilities|Casting|CastToPawn _owner_2))
                        (Utilities|Array|AddUnique (Variables|Default|GetTargets) _aspawn_3))))))))))))
  (return))

(fn FindNearest
  (bind _targets (Variables|Default|GetTargets))
  (LocalVariables|SetCache 1e+09)
  (if (Utilities|Array|IsValidIndex _targets)
    (for _array_element _targets
      (bind _isai_ (Class|BPIPlayerInfo|IsAI?(Message) (Components|GetOwner)))
      (if _isai_
        (bind _isai__2 (Class|BPIPlayerInfo|IsAI?(Message) _array_element))
        (if _isai__2
          _
          (else
            (bind _driver (Class|BPIVehicles|GetDriver(Message) _array_element))
            (Utilities|IsValid _driver
              (:Is%20Valid
                _)))))
      (if (< (Math|Vector|Distance(Vector) (Transformation|GetActorLocation _array_element) (Transformation|GetActorLocation (Components|GetOwner))) (LocalVariables|GetCache))
        (LocalVariables|SetCache (Math|Vector|Distance(Vector) (Transformation|GetActorLocation _array_element) (Transformation|GetActorLocation (Components|GetOwner))))
        (LocalVariables|SetTarget _array_element)))
    (return (LocalVariables|GetTarget))
    (else
      (return 0))))

(fn FindArray
  (return (Utilities|Array|MakeArray "/Game/ModernRPG/Cars/BP_BaseCar.BP_BaseCar_C" "/Game/ModernRPG/General/Blueprints/AI/Blueprints/BP_BaseAI.BP_BaseAI_C" "/Game/ModernRPG/WheeledTank/Blueprint/BP_WheeledTank.BP_WheeledTank_C" "/Game/ModernRPG/Tanks/Blueprints/Base/BP_Tank.BP_Tank_C" "/Game/ModernRPG/Planes/Blueprints/BP_PlaneBase.BP_PlaneBase_C")))

(fn RLType
  (return "NewEnumerator2"))